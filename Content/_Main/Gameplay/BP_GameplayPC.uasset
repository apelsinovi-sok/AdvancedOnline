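; Gameplay player controller that loads the saved player settings and requests the spawn of the selected character.
; On BeginPlay the local controller clears all widgets and reads the PlayerSave slot.
; PassCharacterInfoToServer stores those settings and calls SpawnPlayer on the game mode, reached through a GamePlayGMRefMessage reference getter.
; It also exposes a self-reference getter and an empty chat message event.
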(event `GetChatMessage`
  (params (TextToSend :type Text)))

(event `self.ReceiveBeginPlay`
  (if (`self.IsLocalController`)
    (`WidgetLayoutLibrary.RemoveAllWidgets`)
    (`self.LoadGame`)))

(event `LoadGame`
  (bind _returnvalue (`GameplayStatics.LoadGameFromSlot` (`self.PlayerSettingsSave`)))
  (bind _asplayer_save (cast `/Game/_Main/PlayerSave` _returnvalue))
  (bind _output_get (set `self.Player Settings` (`/Game/_Main/PlayerSave.PlayerInfo` _asplayer_save)))
  (`self.PassCharacterInfoToServer` _output_get))

(event `PassCharacterInfoToServer`
  (params (`Player Settings` :type "/Game/_Main/S_PlayerInfo Structure"))
  (bind _output_get (set `self.Player Settings` `Player Settings`))
  (bind _gameplaygm (message `/Game/_Main/Gameplay/BPI_GamePlayGM.GamePlayGMRef` (`GameplayStatics.GetGameMode`)))
  (`/Game/_Main/Gameplay/BP_GameplayGameMode.SpawnPlayer` _gameplaygm self (`.PlayerCharacter_12_120152FA41C7529643DB36B828707ED5` (break `/Game/_Main/S_PlayerInfo` _output_get))))

(fn `GamePlayPCRef`
  (returns (GamePlayPC :type "/Game/_Main/Gameplay/BP_GameplayPC Object Reference"))
  (return self))

(fn `UserConstructionScript`)