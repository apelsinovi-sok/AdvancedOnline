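; Gameplay game mode that spawns a selected character class for a player controller at a random PlayerStart.
; SpawnPlayer gathers all PlayerStart actors, calls DestroyActor if the controller already has a pawn, then spawns the class at a random start's transform.
; The controller possesses the new actor and the class name is printed.
; GamePlayGMRef returns the game mode itself as a reference.
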(event `SpawnPlayer`
  (params (PlayerController :type "PlayerController Object Reference") (SelectedCharacter :type "Character Class Reference"))
  (bind _spawnpoints (`self.SpawnPoints`))
  ;[1 1 1] Спавн игрока в рандомном месте
  (bind _outactors (`GameplayStatics.GetAllActorsOfClass` "/Script/Engine.PlayerStart"))
  (set `self.SpawnPoints` _outactors)
  (`/Engine/EditorBlueprintResources/StandardMacros.IsValid` (`Controller.K2_GetPawn` PlayerController)
    (:`Is Valid`
      (`self.K2_DestroyActor`))
    (:`Is Not Valid`
      _))
  (bind _returnvalue (`|SpawnActorFromClass` SelectedCharacter (`self.GetTransform` (`|GetArrayItem` _spawnpoints (`KismetMathLibrary.RandomIntegerInRange` 0 (- (`KismetArrayLibrary.Array_Length` _spawnpoints) 1)))) "Undefined" "OverrideRootScale" null null))
  (`Controller.Possess` PlayerController _returnvalue)
  (`KismetSystemLibrary.PrintString` (`KismetSystemLibrary.GetClassDisplayName` SelectedCharacter)))

(fn `GamePlayGMRef`
  (returns (GamePlayGM :type "/Game/_Main/Gameplay/BP_GameplayGameMode Object Reference"))
  (return self))

(fn `UserConstructionScript`)