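; Lobby Game Mode for a multiplayer session, managing connected players, host map settings, character selection and match launch.
; PostLogin registers players and pushes server and map info to their lobby controllers through interface messages.
; EveryoneUpdate rebroadcasts player info, available characters and counts, refreshes the kick list and sets start readiness.
; It also handles kicks, logout cleanup and pawn respawning on character change, then shows loading screens and server-travels to the selected map.
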(event `HostUpdateGameSettings`
  (params (SelectedMapImage :type "Texture2D Object Reference") (SelectedMapName :type Text) (SelectedMapTime :type Text) (SelectedMapID :type Integer))
  ;[1 1 1] Хост внес изменения, уведомить всех в лобби
  (set `self.SelectedMapImage` SelectedMapImage)
  (set `self.SelectedMapName` SelectedMapName)
  (set `self.SelectedMapTime` SelectedMapTime)
  (set `self.SelectedMapID` SelectedMapID)
  (for _array_element (`self.ConnectedPlayers`)
    (bind _lobbypc (message `/Game/_Main/Lobby/BPI_LobbyPC.LobbyPCRef` _array_element))
    (`/Game/_Main/Lobby/BP_LobbyPC.UpdateLobbySetting` _lobbypc (`self.SelectedMapImage`) (`self.SelectedMapName`) (`self.SelectedMapTime`))))

(event `self.K2_PostLogin`
  (params (NewPlayer :type "PlayerController Object Reference"))
  ;[1 1 1] Срабатывает при подключение нового игрока
  (bind _output_get (set `self.ConnectedPlayer` NewPlayer))
  (`KismetArrayLibrary.Array_AddUnique` (`self.ConnectedPlayers`) _output_get)
  (bind _outactors (`GameplayStatics.GetAllActorsOfClass` "/Script/Engine.PlayerStart"))
  (set `self.Spawn Points` _outactors)
  (bind _gameinstance (message `/Game/_Main/BP_GameInstance.SteamGameInstanceRef` (`GameplayStatics.GetGameInstance`)))
  (set `self.Max Players` (`/Game/_Main/SteamGameInstance.MaxPlayers` _gameinstance))
  (set `self.Server Name` (`/Game/_Main/SteamGameInstance.ServerName` _gameinstance))
  (bind _lobbypc (message `/Game/_Main/Lobby/BPI_LobbyPC.LobbyPCRef` (`self.ConnectedPlayer`)))
  (set `self.Lobby PC` _lobbypc)
  (`/Game/_Main/Lobby/BP_LobbyPC.InitialSetup` _lobbypc (`self.Server Name`) (`self.SelectedMapImage`) (`self.SelectedMapName`) (`self.SelectedMapTime`))
  (`self.SpawnPlayer` (`self.ConnectedPlayer`)))

(event `SpawnPlayer`
  (params (Player :type "PlayerController Object Reference")))

(event `EveryoneUpdate`
  (bind _connectedplayers (`self.ConnectedPlayers`))
  ;[1 1 1] Обновляет информацию  в лобби виджета о всех подключенных игроках
  (bind _output_get (set `self.Current Players` (`KismetArrayLibrary.Array_Length` (`self.ConnectedPlayers`))))
  (if (> _output_get 0)
    (`KismetArrayLibrary.Array_Clear` (`self.ConnectedPlayersInfo`))
    (for _array_element _connectedplayers
      (bind _lobbypc (message `/Game/_Main/Lobby/BPI_LobbyPC.LobbyPCRef` _array_element))
      (`KismetArrayLibrary.Array_AddUnique` (`self.ConnectedPlayersInfo`) (`/Game/_Main/Lobby/BP_LobbyPC.PlayerSetting` _lobbypc))
      (`/Game/_Main/Lobby/BP_LobbyPC.UpdateNumberOfPlayers` _lobbypc (`self.Current Players`) (`self.Max Players`)))
    (for _array_element_2 _connectedplayers
      (bind _lobbypc_2 (message `/Game/_Main/Lobby/BPI_LobbyPC.LobbyPCRef` _array_element_2))
      (`/Game/_Main/Lobby/BP_LobbyPC.AddPlayerInfo` _lobbypc_2 (`self.ConnectedPlayersInfo`))
      (`/Game/_Main/Lobby/BP_LobbyPC.UpdateAvailableCharacters` _lobbypc_2 (`self.AvialableCaharacters`))
      (`self.AddToKickList`))
    (for _array_element_3 (`self.ConnectedPlayersInfo`) :!label _label
      (if (== (`.PlayerCharacter_12_120152FA41C7529643DB36B828707ED5` (break `/Game/_Main/S_PlayerInfo` _array_element_3)) null)
        (set `self.CanWeStart?` false)
        (`self.CannotStartGame`)
        (else
          (set `self.CanWeStart?` true))))))

(event `CannotStartGame`
  ;[1 1 1] Обновляет информацию  в лобби виджета о всех подключенных игроках
  (goto _label :!via `Break`))

(event `PlayerKicked`
  (params (PlayerID :type Integer))
  ;[1 1 1] Кик игрока из лобби
  (bind _lobbypc (message `/Game/_Main/Lobby/BPI_LobbyPC.LobbyPCRef` (`|GetArrayItem` (`self.ConnectedPlayers`) PlayerID)))
  (`/Game/_Main/Lobby/BP_LobbyPC.Kicked` _lobbypc))

(event `AddToKickList`
  ;[1 1 1] Добавляет подключенных игроков в список удаления
  (bind _lobbypc (message `/Game/_Main/Lobby/BPI_LobbyPC.LobbyPCRef` (`GameplayStatics.GetPlayerController` 0)))
  (`/Game/_Main/Lobby/BP_LobbyPC.AddPlayerToKickWindow` _lobbypc))

(event `self.K2_OnLogout`
  (params (ExitingController :type "Controller Object Reference"))
  (bind _connectedplayers (`self.ConnectedPlayers`))
  ;[1 1 1] Удаляет игрока из всех массивов и делает персонажа которого он выбрал доступным
  (for (_array_element _array_index) _connectedplayers
    (if (== _array_element ExitingController)
      (break)))
  (bind _lobbypc (message `/Game/_Main/Lobby/BPI_LobbyPC.LobbyPCRef` (`|GetArrayItem` _connectedplayers _array_index)))
  (`KismetArrayLibrary.Array_Set` (`self.AvialableCaharacters`) (`/Game/_Main/Lobby/BP_LobbyPC.SelectedCharacter` _lobbypc))
  (`KismetArrayLibrary.Array_Remove` (`self.ConnectedPlayers`) _array_index)
  (`KismetArrayLibrary.Array_Remove` (`self.ConnectedPlayersInfo`) _array_index)
  (`self.EveryoneUpdate`))

(event `StartLoadingScreen`
  ;[1 1 1] Показывает экран загрузки и загружает карту
  (for _array_element (`self.ConnectedPlayers`)
    (bind _lobbypc (message `/Game/_Main/Lobby/BPI_LobbyPC.LobbyPCRef` _array_element))
    (`/Game/_Main/Lobby/BP_LobbyPC.ShowLoadingScreen` _lobbypc))
  (`self.LaunchGame`))

(event `ChangeCharacter`
  (params (ConnectedPlayer :type "PlayerController Object Reference") (CharacterClass :type "Character Class Reference") (ChangedStatus :type Boolean))
  (bind _spawn_points (`self.Spawn Points`))
  ;[1 1 1] Спавн выбранного игрока
  (if (not ChangedStatus)
    (if (`KismetSystemLibrary.IsValid` (`Controller.K2_GetPawn` ConnectedPlayer))
      (`self.K2_DestroyActor`))
    (bind _returnvalue (`|SpawnActorFromClass` CharacterClass (`self.GetTransform` (`|GetArrayItem` _spawn_points (- (`KismetArrayLibrary.Array_Length` _spawn_points) 1))) "AlwaysSpawn" "OverrideRootScale" null null))
    (`Controller.Possess` ConnectedPlayer _returnvalue)))

(event `LaunchGame`
  (bind _returnvalue (`GameplayStatics.GetPlayerController` 0))
  ;[1 1 1] Показывает экран загрузки и загружает карту
  (switch `int` (`self.SelectedMapID`)
    (:`0`
      (`KismetSystemLibrary.ExecuteConsoleCommand` "servertravel Map-01" _returnvalue))
    (:`1`
      (`KismetSystemLibrary.ExecuteConsoleCommand` "servertravel Map-02" _returnvalue))))

(fn `LobbyGMref`
  (returns (GameGM :type "/Game/_Main/Lobby/BP_LobbyGameMode Object Reference"))
  (return self))

(fn `UserConstructionScript`)